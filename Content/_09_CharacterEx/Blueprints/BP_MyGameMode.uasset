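; BP_MyGameMode is a game mode that manages score, level progress and the player and result screens.
; It adds the player UI at begin play and shows a clear or game-over widget through the GameResult event.
; Every tick it counts all BP_Light actors and sets an Exploding flag when that count equals PassedLights.
; AddScore increments the total score.
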(event Custom|GameResult
  (params (Clear :type Boolean))
  (bind _returnvalue (UserInterface|CreateWidget (select Clear "/Game/_09_CharacterEx/UI/ClearUI.ClearUI_C" "/Game/_09_CharacterEx/UI/GameOverUI.GameOverUI_C")))
  (UserInterface|Viewport|AddtoViewport _returnvalue 0))

(event EventBeginPlay
  (bind _returnvalue (UserInterface|CreateWidget "/Game/_09_CharacterEx/UI/PlayerUI.PlayerUI_C"))
  (UserInterface|Viewport|AddtoViewport _returnvalue 0))

(event EventTick
  (params (DeltaSeconds :type Float%20%28single-precision%29))
  (bind _outactors (Actor|GetAllActorsOfClass "/Game/_09_CharacterEx/Blueprints/BP_Light.BP_Light_C")) ; BP_Light타입의 액터를 모두 찾는다
  (bind _output_get (Variables|Default|SetNumbersOfLights (Utilities|Array|Length _outactors)))
  (if (== _output_get (Variables|Default|GetPassedLights))
    (Variables|Default|SetExploding true)))

(fn ConstructionScript)

(fn AddScore
  (Math|Integer|IncrementInt (Variables|Default|GetTotalScore)))