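; BP_Light is a light actor that switches on when something overlaps its Box and counts toward the game mode's passed-light total.
; The first Box overlap, gated by DoOnce with no check on the overlapping actor, sets Lighting to true and increments PassedLights on BP_MyGameMode.
; Tick applies the Lighting flag to the PointLight's visibility every frame.
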(event OnComponentBeginOverlap(Box)
  (params (OverlappedComponent :type Primitive%20Component%20Object%20Reference) (OtherActor :type Actor%20Object%20Reference) (OtherComp :type Primitive%20Component%20Object%20Reference) (OtherBodyIndex :type Integer) (bFromSweep :type Boolean) (SweepResult :type Hit%20Result%20Structure%20%28by%20ref%29))
  ;[1 1 1] BP_Light의 불을 켠다
  (Utilities|FlowControl|DoOnce false ; 1번만 실행을 한다
    (:Completed
      (Variables|Default|SetLighting true)
      ;[1 1 1] BP_MyGameMode의 PassedLights 변수의 값을 1 증가시킨다
      (bind _asbp_my_game_mode (Utilities|Casting|CastToBP_MyGameMode (Game|GetGameMode)))
      (Variables|/Game/_09_CharacterEx/Blueprints/BP_MyGameMode.BP_MyGameMode_C|SetPassedLights _asbp_my_game_mode (+ (Variables|/Game/_09_CharacterEx/Blueprints/BP_MyGameMode.BP_MyGameMode_C|GetPassedLights _asbp_my_game_mode) 1)))))

(event EventBeginPlay)

(event Collision|EventActorBeginOverlap
  (params (OtherActor :type Actor%20Object%20Reference)))

(event EventTick
  (params (DeltaSeconds :type Float%20%28single-precision%29))
  (Rendering|SetVisibility (Variables|Default|GetPointLight) (Variables|Default|GetLighting) false))

(fn ConstructionScript)