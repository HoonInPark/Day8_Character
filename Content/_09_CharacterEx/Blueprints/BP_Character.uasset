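; Player character Blueprint with camera-yaw-relative movement, a Tab-held speed boost that scales movement input, and jumping tracked by an IsJumping flag.
; AnyDamage briefly swaps the body material and subtracts from Health.
; At zero Health, a one-time death sequence plays sound and particles, swaps the mesh for LizModelDM and applies radius damage to it.
; It then reports a loss to BP_MyGameMode through GameResult.
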(event Custom|Damaged
  (params (Damage :type Float%20%28single-precision%29))
  (Development|PrintString (Utilities|String|Append (Utilities|String|MakeLiteralString "Damaged = ") (Utilities|String|ToString(Float) Damage))))

(event Custom|DamagedBody
  (Rendering|Material|SetMaterial (Variables|Character|GetMesh) 2 "/Game/_09_CharacterEx/Materials/DamagedMaterial.DamagedMaterial")
  (Utilities|FlowControl|Delay 0.5)
  (Rendering|Material|SetMaterial (Variables|Character|GetMesh) 2 "/Game/_09_CharacterEx/Materials/T_Liz_Body_Mat.T_Liz_Body_Mat"))

(event Custom|GameOver
  (bind _asbp_my_game_mode (Utilities|Casting|CastToBP_MyGameMode (Game|GetGameMode)))
  (Default|GameResult _asbp_my_game_mode false))

(event EventOnJumped
  ;[1 1 1] 점프시 IsJumping은 true
  (Variables|Default|SetIsJumping true))

(event EventOnLanded
  (params (Hit :type Hit%20Result%20Structure%20%28by%20ref%29))
  ;[1 1 1] 점프시 IsJumping은 false
  (Variables|Default|SetIsJumping false))

(event Game|Damage|EventAnyDamage
  (params (Damage :type Float%20%28single-precision%29) (DamageType :type Damage%20Type%20Object%20Reference) (InstigatedBy :type Controller%20Object%20Reference) (DamageCauser :type Actor%20Object%20Reference))
  (CallFunction|DamagedBody)
  (bind _output_get (Variables|Default|SetHealth (- (Variables|Default|GetHealth) Damage)))
  (if (<= _output_get 0.0)
    (Utilities|FlowControl|DoOnce false
      (:Completed
        (Audio|PlaySoundatLocation "/Game/_09_CharacterEx/Sound/nogodplease.nogodplease" (Transformation|GetActorLocation) "0, 0, 0" 1.0 1.0 0.0 0 0 0)
        (Rendering|SetVisibility (Variables|Character|GetMesh) false false)
        (Rendering|SetVisibility (Variables|Default|GetLiz_Model_DM) true false)
        (bind _returnvalue (Effects|SpawnEmitteratLocation "/Game/InfinityBladeEffects/Effects/FX_Monsters/FX_Monster_Ausar/P_AU_Trap_Impact.P_AU_Trap_Impact" (Transformation|GetActorLocation)))
        (Utilities|FlowControl|Delay 1.5)
        (Components|DestroyComponent _returnvalue)
        (Class|DestructibleComponent|ApplyRadiusDamage (Variables|Default|GetLiz_Model_DM) 1e+01 (Transformation|GetActorLocation) 1e+01 1e+01 false)
        (Development|PrintString "Dead")
        (CallFunction|GameOver)))))

(event Input|ActionEvents|InputActionJump
  (params (Key :type Key%20Structure :default "None"))
  ;[1 1 1] 점프를 한다
  (:Pressed
    (Character|Jump)))

(event Input|AxisEvents|InputAxisMoveForward
  (params (AxisValue :type Float%20%28single-precision%29))
  ;[1 1 1] 앞뒤로 이동
  (Pawn|Input|AddMovementInput (Math|Vector|GetForwardVector (Math|Rotator|MakeRotator 0.0 0.0 (.Yaw (Math|Rotator|BreakRotator (Pawn|GetControlRotation :!class /Script/Engine.Pawn))))) (* AxisValue (Variables|Default|GetSpeed)) false) ; Movement객체를 사용해서 이동
)

(event Input|AxisEvents|InputAxisMoveRight
  (params (AxisValue :type Float%20%28single-precision%29))
  ;[1 1 1] 좌우로 이동
  (Pawn|Input|AddMovementInput (Math|Vector|GetRightVector (Math|Rotator|MakeRotator 0.0 0.0 (.Yaw (Math|Rotator|BreakRotator (Pawn|GetControlRotation :!class /Script/Engine.Pawn))))) (* AxisValue (Variables|Default|GetSpeed)) false))

(event Input|KeyboardEvents|Tab
  (params (Key :type Key%20Structure :default "None"))
  ;[1 1 1] Tab키를 누르면 Speed변수가 커지고 캐릭터 속도가 향상된다.
  (:Pressed
    (Variables|Default|SetSpeed 1.2))
  (:Released
    (Variables|Default|SetSpeed 0.5)))

(fn ConstructionScript)